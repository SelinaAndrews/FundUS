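; Digsite visualization actor for a mesh loaded from file through its C++ parent (assimp), with visibility, transparency, georeference toggle and deletion controls.
; Users place three colored markers on the mesh, paired with world coordinates and reported to the UI.
; Calibration aligns the markers to those coordinates through a temporary pivot, deriving rotation from three-point bases and uniform scale from one marker distance.
; Marker configurations save to and load from JSON via VaRest and file dialogs.
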(event `self.ReceiveBeginPlay`
  (bind _initialscale (`self.initialScale`))
  (bind _returnvalue (`KismetStringLibrary.ParseIntoArray` (`self.NewFilePath`) "/"))
  ;[1 0.4987 0] Set the filepath in the parent c++ class
  (set `self._filePath` (`KismetSystemLibrary.ConvertToAbsolutePath` (`self.NewFilePath`)))
  ;[1 0.4987 0] Parse filename from filepath
  (set `self.Filename` (`|GetArrayItem` _returnvalue (`KismetArrayLibrary.Array_LastIndex` _returnvalue)))
  ;[1 0.4987 0] apply initial scaling
  (`self.SetActorScale3D` (`KismetMathLibrary.MakeVector` _initialscale _initialscale _initialscale))
  (`self.InitializeMarkers`)
  ;[1 0.4987 0] Disable collision, except for raycasting
  (`PrimitiveComponent.SetCollisionEnabled` (`self._mesh`) "QueryOnly"))

(fn `Add Marker to Mesh`
  (params (SpawnLocation :type "Vector Structure") (MarkerID :type Integer))
  (bind _markerlist (`self.MarkerList`))
  (bind _returnvalue (/ SpawnLocation (`self.initialScale`)))
  (bind _output (`|GetArrayItem` _markerlist MarkerID))
  (bind _output_2 (`|GetArrayItem` (`self.MarkerList`) MarkerID))
  (if (!= MarkerID -1)
    ;[1 0.4987 0] check if marker already exists
    (if (`KismetArrayLibrary.Array_IsValidIndex` (`self.MarkerList`) MarkerID)
      ;[1 0.4987 0] destroy old marker
      (`self.K2_DestroyActor` _output)
      (`KismetArrayLibrary.Array_RemoveItem` _markerlist _output))
    (if (`self.isGeoRefed`)
      ;[1 0.4987 0] add new marker (no active georef.)
      (bind _returnvalue_2 (`|SpawnActorFromClass` "/Game/DigsiteVisualization/Blueprints/Marker.Marker_C" (`KismetMathLibrary.MakeTransform` _returnvalue) "Undefined" "OverrideRootScale" null (`|GetArrayItem` (`self.ColorList`) MarkerID) null))
      (`self.K2_AttachToActor` _returnvalue_2 self "None" "KeepRelative" "KeepRelative" "KeepWorld" true)
      (`KismetArrayLibrary.Array_Set` (`self.MarkerList`) MarkerID _returnvalue_2 true)
      (else
        ;[1 0.4987 0] add new marker (counter georeferencing by adding inverted Transform of WorldSpawn)
        (bind _returnvalue_3 (`|SpawnActorFromClass` "/Game/DigsiteVisualization/Blueprints/Marker.Marker_C" (`KismetMathLibrary.MakeTransform` _returnvalue) "Undefined" "OverrideRootScale" null (`|GetArrayItem` (`self.ColorList`) MarkerID) null))
        (`self.K2_AttachToActor` _returnvalue_3 self "None" "KeepRelative" "KeepRelative" "KeepRelative" true)
        (`self.K2_AddActorWorldTransform` _returnvalue_3 (`KismetMathLibrary.MakeTransform` (`KismetMathLibrary.NegateVector` (`self.SpawnLocation`))) false false)
        (`KismetArrayLibrary.Array_Set` (`self.MarkerList`) MarkerID _returnvalue_3 true)))
    (`KismetSystemLibrary.PrintString` (`KismetStringLibrary.Conv_VectorToString` (`self.K2_GetActorLocation` _output_2)))
    (`KismetSystemLibrary.PrintString` (`KismetStringLibrary.Conv_VectorToString` (`self.GetActorBounds` _output_2 false)))
    (`KismetSystemLibrary.PrintString` "Hello")
    ;[1 0.4987 0] Notify UI about change
    (`/Game/DigsiteVisualization/UserInterface/UserInterface.Marker Updated` (`self.UIRef`) MarkerID)
    (else
      (`KismetSystemLibrary.PrintString` "Marker-ID not set!"))))

(fn `Calibrate by Markers`
  (bind _markerlocationsworld (`self.MarkerLocationsWorld`))
  (bind _uiref (`self.UIRef`))
  (bind _markerlist (`self.MarkerList`))
  (bind _output (`|GetArrayItem` _markerlocationsworld))
  (bind _output_2 (`|GetArrayItem` _markerlocationsworld 1))
  (bind _returnvalue (`self.K2_GetActorLocation` (`|GetArrayItem` _markerlist 1)))
  (bind _returnvalue_2 (`self.K2_GetActorLocation` (`|GetArrayItem` _markerlist)))
  (bind _returnvalue_3 (- _output_2 _output))
  (bind _returnvalue_4 (- _returnvalue _returnvalue_2))
  (bind _returnvalue_5 (`KismetMathLibrary.Cross_VectorVector` _returnvalue_3 (- (`|GetArrayItem` _markerlocationsworld 2) _output)))
  (bind _returnvalue_6 (`KismetMathLibrary.Cross_VectorVector` _returnvalue_4 (- (`self.K2_GetActorLocation` (`|GetArrayItem` _markerlist 2)) _returnvalue_2)))
  (bind _returnvalue_7 (`|SpawnActorFromClass` "/Game/DigsiteVisualization/Blueprints/Pivot.Pivot_C" (`KismetMathLibrary.MakeTransform` (`self.K2_GetActorLocation` (`|GetArrayItem` (`self.MarkerList`)))) "Undefined" "OverrideRootScale" null null))
  (`self.K2_AttachToActor` self _returnvalue_7 "None" "KeepWorld" "KeepWorld" "KeepWorld" true)
  (`self.K2_AddActorWorldTransform` _returnvalue_7 (`KismetMathLibrary.MakeTransform` (- _output _returnvalue_2) (`KismetMathLibrary.NormalizedDeltaRotator` (`KismetMathLibrary.MakeRotationFromAxes` (`KismetMathLibrary.Normal` _returnvalue_3) (`KismetMathLibrary.Normal` (`KismetMathLibrary.Cross_VectorVector` _returnvalue_3 _returnvalue_5)) (`KismetMathLibrary.Normal` _returnvalue_5)) (`KismetMathLibrary.MakeRotationFromAxes` (`KismetMathLibrary.Normal` _returnvalue_4) (`KismetMathLibrary.Normal` (`KismetMathLibrary.Cross_VectorVector` _returnvalue_4 _returnvalue_6)) (`KismetMathLibrary.Normal` _returnvalue_6)))) false false)
  (`self.SetActorScale3D` _returnvalue_7 (`KismetMathLibrary.Conv_DoubleToVector` (/ (`KismetMathLibrary.Vector_Distance` _output _output_2) (`KismetMathLibrary.Vector_Distance` _returnvalue_2 _returnvalue))))
  (`self.K2_DetachFromActor` self "KeepWorld" "KeepWorld" "KeepWorld")
  (`self.K2_DestroyActor` _returnvalue_7)
  (`KismetSystemLibrary.PrintString` "New Position:" true true (struct :`G` 0.66 :`B` 1.0 :`A` 1.0) 10.0)
  (`KismetSystemLibrary.PrintString` (`KismetStringLibrary.Conv_VectorToString` (`self.GetActorBounds` false)) true true (struct :`G` 0.66 :`B` 1.0 :`A` 1.0) 10.0)
  ;[1 0.4987 0] Update UI Marker-TextBoxes
  (`/Game/DigsiteVisualization/UserInterface/UserInterface.Marker Updated` _uiref 0)
  (`/Game/DigsiteVisualization/UserInterface/UserInterface.Marker Updated` _uiref 1)
  (`/Game/DigsiteVisualization/UserInterface/UserInterface.Marker Updated` _uiref 2))

(fn `Delete`
  (bind _uiref (`self.UIRef`))
  (for _array_element (`self.MarkerList`)
    (`self.K2_DestroyActor` _array_element))
  ;[1 0.4987 0] Reset UI Marker-TextBoxes
  (`/Game/DigsiteVisualization/UserInterface/UserInterface.ResetMarker` _uiref 0)
  (`/Game/DigsiteVisualization/UserInterface/UserInterface.ResetMarker` _uiref 1)
  (`/Game/DigsiteVisualization/UserInterface/UserInterface.ResetMarker` _uiref 2)
  (`ActorComponent.K2_DestroyComponent` (`self._mesh`)))

(fn `FocusCamerasOnFG`
  (`/Game/DigsiteVisualization/UserInterface/UserInterface.Set Camera Positions` (`self.UIRef`) (`self.GetActorBounds` false)))

(fn `InitializeMarkers`
  (bind _markerlocationsworld (`self.MarkerLocationsWorld`))
  (bind _uiref (`self.UIRef`))
  (`KismetArrayLibrary.Array_Set` _markerlocationsworld 0 (0.0 0.0 0.0) true)
  (`KismetArrayLibrary.Array_Set` _markerlocationsworld 1 (0.0 0.0 0.0) true)
  (`KismetArrayLibrary.Array_Set` _markerlocationsworld 2 (0.0 0.0 0.0) true)
  (`/Game/DigsiteVisualization/UserInterface/UserInterface.ResetMarker` _uiref 0)
  (`/Game/DigsiteVisualization/UserInterface/UserInterface.ResetMarker` _uiref 1)
  (`/Game/DigsiteVisualization/UserInterface/UserInterface.ResetMarker` _uiref 2))

(fn `LoadMarkerConfiguration`
  (bind _markerlocationsworld (`self.MarkerLocationsWorld`))
  (bind _outfilenames (`EFDFunctionLibrary.OpenFileDialog` "Marker-Konfiguration importieren" "" "" "JSON | *.json" "Single"))
  (if (`KismetArrayLibrary.Array_IsValidIndex` _outfilenames)
    (bind _returnvalue (`IOMarkerConfiguration.readFile` (`|GetArrayItem` _outfilenames)))
    (`KismetSystemLibrary.PrintString` "Flie")
    (`KismetSystemLibrary.PrintString` _returnvalue)
    (bind _returnvalue_2 (`VaRestSubsystem.ConstructVaRestJsonObject` (subsystem `VaRestSubsystem`)))
    (`VaRestJsonObject.DecodeJson` _returnvalue_2 _returnvalue true)
    (`/Game/DigsiteVisualization/UserInterface/UserInterface.UpdateGeoRefButton` (`self.UIRef`) (`VaRestJsonObject.GetBoolField` _returnvalue_2 "isGeoRefed"))
    (bind _returnvalue_3 (`VaRestJsonObject.GetArrayField` _returnvalue_2 "Marker0"))
    (`self.Add Marker to Mesh` (`KismetMathLibrary.MakeVector` (`VaRestJsonValue.AsNumber` (`|GetArrayItem` _returnvalue_3)) (`VaRestJsonValue.AsNumber` (`|GetArrayItem` _returnvalue_3 1)) (`VaRestJsonValue.AsNumber` (`|GetArrayItem` _returnvalue_3 2))))
    (bind _returnvalue_4 (`VaRestJsonObject.GetArrayField` _returnvalue_2 "Marker1"))
    (`self.Add Marker to Mesh` (`KismetMathLibrary.MakeVector` (`VaRestJsonValue.AsNumber` (`|GetArrayItem` _returnvalue_4)) (`VaRestJsonValue.AsNumber` (`|GetArrayItem` _returnvalue_4 1)) (`VaRestJsonValue.AsNumber` (`|GetArrayItem` _returnvalue_4 2))) 1)
    (bind _returnvalue_5 (`VaRestJsonObject.GetArrayField` _returnvalue_2 "Marker2"))
    (`self.Add Marker to Mesh` (`KismetMathLibrary.MakeVector` (`VaRestJsonValue.AsNumber` (`|GetArrayItem` _returnvalue_5)) (`VaRestJsonValue.AsNumber` (`|GetArrayItem` _returnvalue_5 1)) (`VaRestJsonValue.AsNumber` (`|GetArrayItem` _returnvalue_5 2))) 2)
    (bind _returnvalue_6 (`VaRestJsonObject.GetArrayField` _returnvalue_2 "World0"))
    (`KismetArrayLibrary.Array_Set` _markerlocationsworld 0 (`KismetMathLibrary.MakeVector` (`VaRestJsonValue.AsNumber` (`|GetArrayItem` _returnvalue_6)) (`VaRestJsonValue.AsNumber` (`|GetArrayItem` _returnvalue_6 1)) (`VaRestJsonValue.AsNumber` (`|GetArrayItem` _returnvalue_6 2))) true)
    (`/Game/DigsiteVisualization/UserInterface/UserInterface.Marker Updated` (`self.UIRef`) 0)
    (bind _returnvalue_7 (`VaRestJsonObject.GetArrayField` _returnvalue_2 "World1"))
    (`KismetArrayLibrary.Array_Set` _markerlocationsworld 1 (`KismetMathLibrary.MakeVector` (`VaRestJsonValue.AsNumber` (`|GetArrayItem` _returnvalue_7)) (`VaRestJsonValue.AsNumber` (`|GetArrayItem` _returnvalue_7 1)) (`VaRestJsonValue.AsNumber` (`|GetArrayItem` _returnvalue_7 2))) true)
    (`/Game/DigsiteVisualization/UserInterface/UserInterface.Marker Updated` (`self.UIRef`) 1)
    (bind _returnvalue_8 (`VaRestJsonObject.GetArrayField` _returnvalue_2 "World2"))
    (`KismetArrayLibrary.Array_Set` _markerlocationsworld 2 (`KismetMathLibrary.MakeVector` (`VaRestJsonValue.AsNumber` (`|GetArrayItem` _returnvalue_8)) (`VaRestJsonValue.AsNumber` (`|GetArrayItem` _returnvalue_8 1)) (`VaRestJsonValue.AsNumber` (`|GetArrayItem` _returnvalue_8 2))) true)
    (`/Game/DigsiteVisualization/UserInterface/UserInterface.Marker Updated` (`self.UIRef`) 2)))

(fn `SaveMarkerConfiguration`
  (bind _returnvalue (subsystem `VaRestSubsystem`))
  (bind _returnvalue_2 (subsystem `VaRestSubsystem`))
  (bind _markerlocationsworld (`self.MarkerLocationsWorld`))
  (bind _markerlist (`self.MarkerList`))
  (bind (_output_x _output_y _output_z) (`KismetMathLibrary.BreakVector` (`|GetArrayItem` _markerlocationsworld 2)))
  (bind (_output_x_2 _output_y_2 _output_z_2) (`KismetMathLibrary.BreakVector` (`|GetArrayItem` _markerlocationsworld)))
  (bind (_output_x_3 _output_y_3 _output_z_3) (`KismetMathLibrary.BreakVector` (`|GetArrayItem` _markerlocationsworld 1)))
  (bind (_returnvalue_x _returnvalue_y _returnvalue_z) (`KismetMathLibrary.BreakVector` (`self.K2_GetActorLocation` (`|GetArrayItem` _markerlist))))
  (bind (_returnvalue_x_2 _returnvalue_y_2 _returnvalue_z_2) (`KismetMathLibrary.BreakVector` (`self.K2_GetActorLocation` (`|GetArrayItem` _markerlist 1))))
  (bind (_returnvalue_x_3 _returnvalue_y_3 _returnvalue_z_3) (`KismetMathLibrary.BreakVector` (`self.K2_GetActorLocation` (`|GetArrayItem` _markerlist 2))))
  (bind _returnvalue_3 (`VaRestSubsystem.ConstructVaRestJsonObject` _returnvalue_2))
  (set `self.Json` _returnvalue_3)
  (`VaRestJsonObject.SetField` (`self.Json`) "isGeoRefed" (`VaRestSubsystem.ConstructJsonValueBool` _returnvalue_2 (`self.isGeoRefed`)))
  (`VaRestJsonObject.SetField` (`self.Json`) "Marker0" (`VaRestSubsystem.ConstructJsonValueArray` _returnvalue_2 (`|MakeArray` (`VaRestSubsystem.ConstructJsonValueNumber` _returnvalue_2 _returnvalue_x) (`VaRestSubsystem.ConstructJsonValueNumber` _returnvalue_2 _returnvalue_y) (`VaRestSubsystem.ConstructJsonValueNumber` _returnvalue_2 _returnvalue_z))))
  (`VaRestJsonObject.SetField` (`self.Json`) "Marker1" (`VaRestSubsystem.ConstructJsonValueArray` _returnvalue_2 (`|MakeArray` (`VaRestSubsystem.ConstructJsonValueNumber` _returnvalue_2 _returnvalue_x_2) (`VaRestSubsystem.ConstructJsonValueNumber` _returnvalue_2 _returnvalue_y_2) (`VaRestSubsystem.ConstructJsonValueNumber` _returnvalue_2 _returnvalue_z_2))))
  (`VaRestJsonObject.SetField` (`self.Json`) "Marker2" (`VaRestSubsystem.ConstructJsonValueArray` _returnvalue_2 (`|MakeArray` (`VaRestSubsystem.ConstructJsonValueNumber` _returnvalue_2 _returnvalue_x_3) (`VaRestSubsystem.ConstructJsonValueNumber` _returnvalue_2 _returnvalue_y_3) (`VaRestSubsystem.ConstructJsonValueNumber` _returnvalue_2 _returnvalue_z_3))))
  (`VaRestJsonObject.SetField` (`self.Json`) "World0" (`VaRestSubsystem.ConstructJsonValueArray` _returnvalue (`|MakeArray` (`VaRestSubsystem.ConstructJsonValueNumber` _returnvalue _output_x_2) (`VaRestSubsystem.ConstructJsonValueNumber` _returnvalue _output_y_2) (`VaRestSubsystem.ConstructJsonValueNumber` _returnvalue _output_z_2))))
  (`VaRestJsonObject.SetField` (`self.Json`) "World1" (`VaRestSubsystem.ConstructJsonValueArray` _returnvalue (`|MakeArray` (`VaRestSubsystem.ConstructJsonValueNumber` _returnvalue _output_x_3) (`VaRestSubsystem.ConstructJsonValueNumber` _returnvalue _output_y_3) (`VaRestSubsystem.ConstructJsonValueNumber` _returnvalue _output_z_3))))
  (`VaRestJsonObject.SetField` (`self.Json`) "World2" (`VaRestSubsystem.ConstructJsonValueArray` _returnvalue (`|MakeArray` (`VaRestSubsystem.ConstructJsonValueNumber` _returnvalue _output_x) (`VaRestSubsystem.ConstructJsonValueNumber` _returnvalue _output_y) (`VaRestSubsystem.ConstructJsonValueNumber` _returnvalue _output_z))))
  (bind (_outfilenames _returnvalue_4) (`EFDFunctionLibrary.SaveFileDialog` "Marker-Konfiguration speichern" "" (`KismetStringLibrary.Concat_StrStr` "FundUS-FGConfig_" (`KismetStringLibrary.Split` (`self.Filename`) ".")) "" "json" "Single"))
  (if _returnvalue_4
    (`IOMarkerConfiguration.saveFile` (`VaRestJsonObject.EncodeJsonToSingleString` (`self.Json`)) (`|GetArrayItem` _outfilenames))))

(fn `ToggleGoeref`
  (params (isGeoref :type Boolean))
  (bind _output_get (set `self.isGeoRefed` isGeoref))
  (if _output_get
    (`self.K2_SetActorLocation` (0.0 0.0 0.0) false true)
    (`KismetSystemLibrary.PrintString` "do georef")
    (else
      (`self.K2_SetActorLocation` (`self.SpawnLocation`) false true)
      (`KismetSystemLibrary.PrintString` "no georef"))))

(fn `ToggleVisibility`
  (bind _returnvalue (not (`self.IsVisible`)))
  (`self.SetActorHiddenInGame` _returnvalue)
  (for _array_element (`self.MarkerList`)
    (`self.SetActorHiddenInGame` _array_element _returnvalue))
  (set `self.IsVisible` _returnvalue))

(fn `UpdateTransparency`
  (params (NewTransparency :type "Float (double-precision)"))
  (`MeshComponent.SetScalarParameterValueOnMaterials` (`self._mesh`) "Transparency" NewTransparency))

(fn `UserConstructionScript`)