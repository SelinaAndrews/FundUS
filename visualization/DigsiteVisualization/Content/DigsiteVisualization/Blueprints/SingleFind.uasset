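; SingleFind is an actor for one find in a digsite visualization, shown as a billboard sprite with a clickable sphere.
; On BeginPlay it binds a setup event that picks the sprite from nested string switches on Identification, falling back to Definition, then Basic Form, with special branches for some codes.
; Clicking the visible sphere opens the find's info box and applies a selected material.
; An older sprite-selection switch remains unconnected.
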(event `self.ReceiveBeginPlay`
  (add `self.Setup` (delegate `VisualizationSetup`)))

(event `VisualizationSetup`
  (bind _billboard (`self.Billboard`))
  (bind _billboard_2 (`self.Billboard`))
  (bind _billboard_3 (`self.Billboard`))
  ;[1 1 1] Check the Identification String for the listed entries
  (switch `string` (`self.identification`)
    (:`Default`
      ;[1 1 1] If no Identification applies, check the Definition string
      (switch `string` (`self.definition`)
        (:`Default`
          ;[1 1 1] If no Definition applies, check the Basic Form string
          (switch `string` (`self.basic_form`)
            (:`Default`
              ;[1 1 1] Set sprites according to Basic Form
              (`BillboardComponent.SetSprite` _billboard_3 "/Game/DigsiteVisualization/Materials/Symbols_small/misc.misc" :!label _label))
            (:`AB`
              (`BillboardComponent.SetSprite` _billboard_3 "/Game/DigsiteVisualization/Materials/Symbols_small/AB.AB" :!label _label_2))
            (:`AS`
              (`BillboardComponent.SetSprite` _billboard_3 "/Game/DigsiteVisualization/Materials/Symbols_small/AS.AS" :!label _label_3))
            (:`KL`
              (`BillboardComponent.SetSprite` _billboard_3 "/Game/DigsiteVisualization/Materials/Symbols_small/KL.KL" :!label _label_4))
            (:`LA`
              (`BillboardComponent.SetSprite` _billboard_3 "/Game/DigsiteVisualization/Materials/Symbols_small/LA.LA" :!label _label_5))))
        (:`LVAB`
          ;[1 1 1] Set sprites according to Definition
          (`BillboardComponent.SetSprite` _billboard_2 "/Game/DigsiteVisualization/Materials/Symbols_small/LVAB.LVAB" :!label _label_6))
        (:`LVKL`
          (`BillboardComponent.SetSprite` _billboard_2 "/Game/DigsiteVisualization/Materials/Symbols_small/LVKL.LVKL" :!label _label_7))
        (:`KLKE`
          (`BillboardComponent.SetSprite` _billboard_2 "/Game/DigsiteVisualization/Materials/Symbols_small/KLKE.KLKE" :!label _label_8))
        (:`LAKE`
          (`BillboardComponent.SetSprite` _billboard_2 "/Game/DigsiteVisualization/Materials/Symbols_small/LAKE.LAKE" :!label _label_9))
        (:`LVKE`
          (`BillboardComponent.SetSprite` _billboard_2 "/Game/DigsiteVisualization/Materials/Symbols_small/LVKE.LVKE" :!label _label_10))
        (:`KR`
          (`BillboardComponent.SetSprite` _billboard_2 "/Game/DigsiteVisualization/Materials/Symbols_small/KR.KR" :!label _label_11))
        (:`ST`
          (`BillboardComponent.SetSprite` _billboard_2 "/Game/DigsiteVisualization/Materials/Symbols_small/ST.ST" :!label _label_12))
        (:`SPKL`
          (`BillboardComponent.SetSprite` _billboard_2 "/Game/DigsiteVisualization/Materials/Symbols_small/SPKL.SPKL" :!label _label_13))
        (:`SC`
          (`BillboardComponent.SetSprite` _billboard_2 "/Game/DigsiteVisualization/Materials/Symbols_small/SC.SC" :!label _label_14))
        (:`SP`
          (`BillboardComponent.SetSprite` _billboard_2 "/Game/DigsiteVisualization/Materials/Symbols_small/SP.SP" :!label _label_15))
        (:`BI`
          (`BillboardComponent.SetSprite` _billboard_2 "/Game/DigsiteVisualization/Materials/Symbols_small/BI.BI" :!label _label_16))))
    (:`KN`
      ;[1 1 1] Set sprites according to Identification only
      (`BillboardComponent.SetSprite` _billboard "/Game/DigsiteVisualization/Materials/Symbols_small/KN.KN"))
    (:`GE`
      (`BillboardComponent.SetSprite` _billboard "/Game/DigsiteVisualization/Materials/Symbols_small/GE.GE"))
    (:`KER`
      (`BillboardComponent.SetSprite` _billboard "/Game/DigsiteVisualization/Materials/Symbols_small/KER.KER" :!label _label_17))
    (:`MET`
      (goto _label_17))
    (:`PL`
      (goto _label_17))
    (:`GL`
      (goto _label_17))
    (:`ZN`
      (`BillboardComponent.SetSprite` _billboard "/Game/DigsiteVisualization/Materials/Symbols_small/ZN.ZN"))
    (:`EB`
      (`BillboardComponent.SetSprite` _billboard "/Game/DigsiteVisualization/Materials/Symbols_small/EB.EB"))
    (:`GF`
      ;[1 1 1] For the Identification "GF" check the Definition String for the listed entries
      (switch `string` (`self.definition`)
        (:`Default`
          ;[1 1 1] For the Identification "GF", if no Definition applies, check the Basic Form string for the listed entries
          (switch `string` (`self.basic_form`)
            (:`Default`
              (goto _label))
            (:`AB`
              (goto _label_2))
            (:`AS`
              (goto _label_3))
            (:`KL`
              (goto _label_4))
            (:`LA`
              (goto _label_5))))
        (:`LVAB`
          (goto _label_6))
        (:`LVKL`
          (goto _label_7))
        (:`KR`
          (goto _label_11))
        (:`ST`
          (goto _label_12))
        (:`SPKL`
          (goto _label_13))
        (:`SC`
          (goto _label_14))
        (:`SP`
          (goto _label_15))
        (:`BI`
          (goto _label_16))))
    (:`KE`
      ;[1 1 1] For the Identification "KE" check the Definition string
      (switch `string` (`self.definition`)
        (:`Default`
          ;[1 1 1] Set sprite according to Definition
          (`BillboardComponent.SetSprite` (`self.Billboard`) "/Game/DigsiteVisualization/Materials/Symbols_small/KE.KE"))
        (:`KLKE`
          (goto _label_8))
        (:`LAKE`
          (goto _label_9))
        (:`LVKE`
          (goto _label_10))))
    (:`SI`
      ;[1 1 1] Set sprite according to Identification only
      (`BillboardComponent.SetSprite` (`self.Billboard`) "/Game/DigsiteVisualization/Materials/Symbols_small/Silex.Silex"))))

(event `self.Sphere.OnClicked`
  (params (TouchedComponent :type "PrimitiveComponent Object Reference") (ButtonPressed :type "Key Structure"))
  ;[1 1 1] Show the according info box if a visible click sphere is clicked
  (if (not (`self.bHidden`))
    (`/Game/DigsiteVisualization/UserInterface/UserInterface.ShowSingleFindInfoBox` (`self.UserInterface`) self)
    (`PrimitiveComponent.SetMaterial` (`self.Sphere`) 0 "/Engine/EditorMaterials/PhAT_ElemSelectedMaterial.PhAT_ElemSelectedMaterial")))

(fn `UserConstructionScript`)