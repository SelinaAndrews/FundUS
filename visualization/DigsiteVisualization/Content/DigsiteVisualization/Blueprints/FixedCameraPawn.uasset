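; Camera pawn for the digsite visualization, controlled by mouse through a spring arm.
; Holding the right mouse button applies Turn and LookUp as controller yaw and pitch, while the Zoom axis changes the arm length without letting it go below zero.
; An orthographic mode scales all three inputs by its own control factor.
; BeginPlay stores the starting position and rotation, which this graph does not use further.
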(event `self.ReceiveBeginPlay`
  ;[1 1 1] Save Start Position on BeginPlay
  (set `self.StartPosition` (`self.K2_GetActorLocation`))
  (set `self.StartRotation` (`self.K2_GetActorRotation`)))

(event `InputAxis|Turn`
  (params (AxisValue :type "Float (single-precision)"))
  ;[1 1 1] Get Movement from Mouse when Right Mouse Button is pressed, scaling for Orthographic Mode when activated
  (if (`PlayerController.IsInputKeyDown` (`GameplayStatics.GetPlayerController` 0) "RightMouseButton")
    (if (`self.OrthographicMode`)
      (`self.AddControllerYawInput` (* AxisValue (`self.OrthographicControlScale`)))
      (else
        (`self.AddControllerYawInput` AxisValue)))))

(event `InputAxis|LookUp`
  (params (AxisValue :type "Float (single-precision)"))
  ;[1 1 1] Get Movement from Mouse when Right Mouse Button is pressed, scaling for Orthographic Mode when activated
  (if (`PlayerController.IsInputKeyDown` (`GameplayStatics.GetPlayerController` 0) "RightMouseButton")
    (if (`self.OrthographicMode`)
      (`self.AddControllerPitchInput` (* AxisValue (`self.OrthographicControlScale`)))
      (else
        (`self.AddControllerPitchInput` AxisValue)))))

(event `InputAxis|Zoom`
  (params (AxisValue :type "Float (single-precision)"))
  (bind _springarm (`self.SpringArm`))
  (bind _springarm_2 (`self.SpringArm`))
  (bind _returnvalue (+ (* AxisValue -10.0) (`SpringArmComponent.TargetArmLength` _springarm)))
  (bind _returnvalue_2 (+ (* (* AxisValue (`self.OrthographicControlScale`)) -10.0) (`SpringArmComponent.TargetArmLength` _springarm_2)))
  (if (`self.OrthographicMode`)
    ;[1 1 1] Set Spring Arm Length to new zoom level as input by the scroll wheel multiplied with the orthographic scale if this is greater than 0
    (`/Engine/EditorBlueprintResources/StandardMacros.CompareFloat` _returnvalue_2
      (:`>`
        _)
      (:`==`
        _))
    (set `SpringArmComponent.TargetArmLength` _returnvalue_2 _springarm_2)
    (else
      ;[1 1 1] Set Spring Arm Length to new zoom level as input by the scroll wheel if this is greater than 0
      (`/Engine/EditorBlueprintResources/StandardMacros.CompareFloat` _returnvalue
        (:`>`
          _)
        (:`==`
          _))
      (set `SpringArmComponent.TargetArmLength` _returnvalue _springarm))))

(fn `UserConstructionScript`)