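; Import handler in the digsite visualization that lets the user load an FG model from disk into the world.
; On BeginPlay it binds to the StartFileDialog dispatcher, which opens a single-select file dialog for FBX or PLY files.
; A chosen file spawns a ProceduralEntityBlueprint at the supplied location with the file path and scale.
; It then notifies the calling UI through its MeshCreated dispatch.
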(event `self.ReceiveBeginPlay`
  (add `self.StartFileDialog` (delegate `OpenFileDialog Dispatch`)))

(event `OpenFileDialog Dispatch` :!signature `self.StartFileDialog`
  (params (SpawnLocation :type "Vector Structure") (UIRef :type "/Game/DigsiteVisualization/UserInterface/UserInterface Object Reference"))
  (bind _outfilenames (`EFDFunctionLibrary.OpenFileDialog` "Import FG" "" "" "FBX | *.fbx|PLY |*.ply" "Single"))
  (if (`KismetArrayLibrary.Array_IsValidIndex` _outfilenames)
    (bind _returnvalue (`|SpawnActorFromClass` :`Class` "/Game/DigsiteVisualization/Blueprints/ProceduralEntityBlueprint.ProceduralEntityBlueprint_C" :`SpawnTransform` (`KismetMathLibrary.MakeTransform` SpawnLocation) :`CollisionHandlingOverride` "Undefined" :`TransformScaleMethod` "OverrideRootScale" :`NewFilePath` (`|GetArrayItem` _outfilenames) :`UIRef` UIRef :`SpawnLocation` SpawnLocation :`initialScale` (`self.scale`) :`Instigator` null))
    (`KismetSystemLibrary.PrintString` "Spawned FG at:")
    (`KismetSystemLibrary.PrintString` (`KismetStringLibrary.Conv_VectorToString` SpawnLocation))
    (`/Game/DigsiteVisualization/UserInterface/UserInterface.MeshCreatedDispatch` UIRef _returnvalue) ; Tells the ui, that the mesh has been successfully created.
  ))

(fn `UserConstructionScript`)