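; CameraController is a controller Blueprint that handles mouse-click marker placement on procedural meshes in the digsite visualization.
; When left mouse is released during marker placement mode, it runs a complex Visibility trace under the cursor.
; A hit on a ProceduralEntityBlueprint adds the current marker at that location, exits placement mode, clears the marker ID and prints debug info.
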(event `Key|LeftMouseButton`
  (params (Key :type "Key Structure"))
  (bind (_hitresult _returnvalue) (`self.GetHitResultUnderCursorByChannel` "TraceTypeQuery1"))
  (bind (_bblockinghit _binitialoverlap _time _distance _location _impactpoint _normal _impactnormal _physmat _hitactor) (`GameplayStatics.BreakHitResult` _hitresult))
  ;[1 0.4987 0] Get Mouse HIts on FG
  (:`Released`
    (if (`self.MarkerPlacementMode`)
      (if _returnvalue
        (bind _asprocedural_entity_blueprint (cast `/Game/DigsiteVisualization/Blueprints/ProceduralEntityBlueprint` _hitactor))
        (`/Game/DigsiteVisualization/Blueprints/ProceduralEntityBlueprint.Add Marker to Mesh` _asprocedural_entity_blueprint _location (`self.currentMarker`))
        (set `self.MarkerPlacementMode` false)
        (set `self.currentMarker` -1)
        (`KismetSystemLibrary.PrintString` "added marker")
        (`KismetSystemLibrary.PrintString` (`KismetStringLibrary.Conv_VectorToString` _location))
        (`KismetSystemLibrary.PrintString` (`/Game/DigsiteVisualization/Blueprints/ProceduralEntityBlueprint.Filename` _asprocedural_entity_blueprint))))))

(fn `UserConstructionScript`)